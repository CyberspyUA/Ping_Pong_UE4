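; BP_GateActor is a ping-pong gate that gives visual and audio feedback when it is struck.
; On BeginPlay it creates a dynamic instance of the gate material on its static mesh.
; ReacttoStrike tints the material cyan, plays the goal-score sound and calls ReactToStrikeCPP.
; After a brief delay it sets the color to white.
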(event `self.ReceiveBeginPlay`
  (bind _returnvalue (`PrimitiveComponent.CreateDynamicMaterialInstance` (`self.StaticMesh`) 0 "/Game/Materials/M_Gate_Inst.M_Gate_Inst" "None"))
  (set `self.DynamicMaterial` _returnvalue))

(event `self.ReactToStrike`
  (bind _dynamicmaterial (`self.DynamicMaterial`))
  (`MaterialInstanceDynamic.SetVectorParameterValue` _dynamicmaterial "Color" (struct :`G` 0.957898 :`B` 1.0 :`A` 1.0))
  (`GameplayStatics.SpawnSoundAtLocation` "/Game/Sounds/Goal_Score_Cue.Goal_Score_Cue" (`KismetMathLibrary.Conv_IntVectorToVector` (`GameplayStatics.GetWorldOriginLocation`)) (struct) 1.0 1.0 0.0 null null)
  (`self.ReactToStrike_CPP`)
  (`KismetSystemLibrary.Delay` 0.2)
  (`MaterialInstanceDynamic.SetVectorParameterValue` _dynamicmaterial "Color" (struct :`R` 1.0 :`G` 1.0 :`B` 1.0 :`A` 1.0)))

(fn `UserConstructionScript`)